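; BP_MagnetShooter is a pickup weapon that spawns a BP_MagneticField where its shot hits.
; Overlapping its capsule while it is unowned attaches it to the first-person character's mesh at GripPoint, adds it to Equipments, adds the weapons input context and shows an aim widget.
; Use activates the beam effect and traces from the gun toward a ranged point along the owner's camera forward, spawning the field at the impact.
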(event OnComponentBeginOverlap(CapsuleTrigger)
  (params (OverlappedComponent :type Primitive%20Component%20Object%20Reference) (OtherActor :type Actor%20Object%20Reference) (OtherComp :type Primitive%20Component%20Object%20Reference) (OtherBodyIndex :type Integer) (bFromSweep :type Boolean) (SweepResult :type Hit%20Result%20Structure%20%28by%20ref%29))
  (bind _asbp_first_person_character (|IfAttachablereturnBP_FPCharacter OtherActor)
    (:else
      (|AttachtoCharacter _asbp_first_person_character)
      (bind _returnvalue (UserInterface|CreateWidget "/Game/UI/Player/PlayerUI_Aim.PlayerUI_Aim_C"))
      (UserInterface|Viewport|AddtoViewport _returnvalue 0))))

(event EventBeginPlay)

(event Collision|EventActorBeginOverlap
  (params (OtherActor :type Actor%20Object%20Reference)))

(event EventTick
  (params (DeltaSeconds :type Float%20%28single-precision%29)))

(event EventUse
  (bind _equipmentowner (Variables|Default|GetEquipmentOwner))
  (bind _as폰 (Utilities|Casting|CastToPawn _equipmentowner))
  (bind _returnvalue (Actor|GetComponentbyClass _as폰 "/Script/Engine.CameraComponent"))
  (Components|Activation|Activate (Variables|Default|GetFX_Beam) false)
  (bind (_outhit _returnvalue_2) (Collision|LineTraceByChannel (Transformation|GetWorldLocation (Variables|Default|GetSM_Gun)) (+ (Transformation|GetWorldLocation _returnvalue) (* (Math|Vector|GetForwardVector _returnvalue) (Variables|Default|GetRange))) "TraceTypeQuery1" false 0 "ForOneFrame"))
  (if _returnvalue_2
    (Game|SpawnActorfromClass "/Game/Blueprints/Weapon/BP_MagneticField.BP_MagneticField_C" (Math|Conversions|ToTransform(Vector) (.Location (Collision|BreakHitResult _outhit))) "Undefined" 0 0)))

(fn ConstructionScript)